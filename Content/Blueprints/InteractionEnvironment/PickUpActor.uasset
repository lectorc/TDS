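; Base pickup actor for dropped weapons or items that TDS123Character can collect.
; Sphere overlap passes the character's InventoryComponent to OverlapCharacter, an empty event here, and PickUpSuccess destroys the actor.
; InitActor applies the static mesh from the supplied info, falling back to the skeletal mesh, destroys the unused mesh component, and prints an error if neither exists.
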(event OnComponentBeginOverlap(Sphere1)
  (params (OverlappedComponent :type Primitive%20Component%20Object%20Reference) (OtherActor :type Actor%20Object%20Reference) (OtherComp :type Primitive%20Component%20Object%20Reference) (OtherBodyIndex :type Integer) (bFromSweep :type Boolean) (SweepResult :type Hit%20Result%20Structure%20%28by%20ref%29))
  (bind _astds123character (Utilities|Casting|CastToTDS123Character OtherActor))
  (CallFunction|OverlapCharacter (Variables|/Script/TDS123.TDS123Character|GetInventoryComponent _astds123character)))

(event Custom|OverlapCharacter
  (params (ToInventory :type TDS123%20Inventory%20Component%20Object%20Reference)))

(event EventBeginPlay)

(event Collision|EventActorBeginOverlap
  (params (OtherActor :type Actor%20Object%20Reference)))

(event EventTick
  (params (DeltaSeconds :type Float%20%28single-precision%29)))

(fn ConstructionScript)

(fn PickUpSuccess
  (Actor|DestroyActor))

(fn InitActor
  (params (InfoActor :type Drop%20Item%20Structure))
  (bind (_weaponstaticmesh _weaponskeletmesh) (Utilities|Struct|BreakDropItem InfoActor))
  (Utilities|IsValid _weaponstaticmesh
    (:Is%20Valid
      (Components|DestroyComponent (Variables|Default|GetSkeletalMesh))
      (Components|StaticMesh|SetStaticMesh (Variables|Default|GetStaticMesh) _weaponstaticmesh))
    (:Is%20Not%20Valid
      (Utilities|IsValid _weaponskeletmesh
        (:Is%20Valid
          (Components|DestroyComponent (Variables|Default|GetStaticMesh))
          (Components|SkeletalMesh|SetSkeletalMeshAsset (Variables|Default|GetSkeletalMesh) _weaponskeletmesh))
        (:Is%20Not%20Valid
          (Development|PrintString "ERROR Drop Item Has No Mesh"))))))