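; CanDamageActor is a damageable world object that shows damage feedback and explodes when its health runs out.
; AnyDamage feeds damage into the TDS123Health component, while point and radial damage events only print debug output.
; Health changes spawn a DisplayDamageActor at a randomly jittered offset, initialized with damage and current health.
; The death callback destroys the actor and spawns an explosion sound and particle effect at its location.
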(event Custom|OnHealthChange_Event
  (params (Health :type Float%20%28single-precision%29) (Damage :type Float%20%28single-precision%29))
  (bind _returnvalue (Game|SpawnActorfromClass "/Game/Blueprints/InteractionEnvironment/DisplayDamage/DisplayDamageActor.DisplayDamageActor_C" (Math|Transform|MakeTransform (+ (+ (Math|Vector|MakeVector (Math|Random|RandomFloatinRange -1e+01 1e+01) (Math|Random|RandomFloatinRange -1e+01 1e+01) 0.0) (Variables|Default|GetLocalPointSpawnHealthNumber)) (Transformation|GetActorLocation))) "AlwaysSpawn" "MultiplyWithRoot" 0 0))
  (Default|InitActor _returnvalue Damage Health))

(event Custom|OnDead_Event
  (Actor|DestroyActor))

(event EventBeginPlay
  (bind _tds123_health (Variables|Default|GetTDS123_Health))
  (EventDispatchers|BindEventtoOnHealthChange _tds123_health (delegate Custom|OnHealthChange_Event))
  (EventDispatchers|BindEventtoOnDead _tds123_health (delegate Custom|OnDead_Event)))

(event Game|Damage|EventAnyDamage
  (params (Damage :type Float%20%28single-precision%29) (DamageType :type Damage%20Type%20Object%20Reference) (InstigatedBy :type Controller%20Object%20Reference) (DamageCauser :type Actor%20Object%20Reference))
  (Development|PrintString (Utilities|String|ToString(Float) Damage))
  (Class|TDS123HealthComponent|ReceiveDamage (Variables|Default|GetTDS123_Health) Damage))

(event Game|Damage|EventPointDamage
  (params (Damage :type Float%20%28single-precision%29) (DamageType :type Damage%20Type%20Object%20Reference) (HitLocation :type Vector :default "0, 0, 0") (HitNormal :type Vector :default "0, 0, 0") (HitComponent :type Primitive%20Component%20Object%20Reference) (BoneName :type Name :default "None") (ShotFromDirection :type Vector :default "0, 0, 0") (InstigatedBy :type Controller%20Object%20Reference) (DamageCauser :type Actor%20Object%20Reference) (HitInfo :type Hit%20Result%20Structure%20%28by%20ref%29))
  (Development|PrintString (Utilities|String|ToString(Float) Damage)))

(event Game|Damage|EventRadialDamage
  (params (DamageReceived :type Float%20%28single-precision%29) (DamageType :type Damage%20Type%20Object%20Reference) (Origin :type Vector :default "0, 0, 0") (HitInfo :type Hit%20Result%20Structure%20%28by%20ref%29) (InstigatedBy :type Controller%20Object%20Reference) (DamageCauser :type Actor%20Object%20Reference))
  (Development|PrintString "Hello" true true "(R=0.000000,G=0.660000,B=1.000000,A=1.000000)" DamageReceived))

(fn ConstructionScript)

(fn DestroyActor
  (bind _returnvalue (Transformation|GetActorLocation))
  (Actor|DestroyActor)
  (Audio|SpawnSoundatLocation "/Game/MilitaryWeapDark/Sound/GrenadeLauncher/Wavs/GrenadeLauncher_Explosion01.GrenadeLauncher_Explosion01" _returnvalue "0, 0, 0" 1.0 1.0 0.0 0 0)
  (Effects|SpawnEmitteratLocation "/Game/FX_Effects/Particles/P_Explosion.P_Explosion" _returnvalue))