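; Ammo pickup actor that adds rifle, shotgun or grenade launcher ammo to an overlapping character's inventory.
; On BeginPlay, InitActor uses the weapon ammo type to pick the static mesh and Niagara effect, destroying either component when its validity check fails.
; The parent's OverlapCharacter event is extended to check that the inventory can take that ammo, add the count and call PickUpSuccess.
; A debug "Hello" print remains in the overlap event.
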(event EventBeginPlay
  (|CallParentFunction)
  (CallFunction|InitActor))

(event Collision|EventActorBeginOverlap
  (params (OtherActor :type Actor%20Object%20Reference))
  (|CallParentFunction OtherActor) ; This node is disabled and will not be called.\nDrag off pins to build functionality.
)

(event EventTick
  (params (DeltaSeconds :type Float%20%28single-precision%29))
  (|CallParentFunction DeltaSeconds) ; This node is disabled and will not be called.\nDrag off pins to build functionality.
)

(event EventOverlapCharacter
  (params (ToInventory :type TDS123%20Inventory%20Component%20Object%20Reference))
  (bind _weapontypeammo (Variables|Default|GetWeaponTypeAmmo))
  (Development|PrintString "Hello")
  (|CallParentFunction ToInventory)
  (bind _returnvalue (Class|TDS123InventoryComponent|CheckCanTakeAmmo ToInventory _weapontypeammo))
  (if _returnvalue
    (Class|TDS123InventoryComponent|AmmoSlotChangeValue ToInventory _weapontypeammo (Variables|Default|GetCout))
    (CallFunction|PickUpSuccess)))

(fn ConstructionScript
  (|CallParentFunction))

(fn InitActor
  (bind _staticmesh (Variables|Default|GetStaticMesh))
  (bind _niagara (Variables|Default|GetNiagara))
  (bind _weapontypeammo (Variables|Default|GetWeaponTypeAmmo))
  (bind _returnvalue (Utilities|Select :Index _weapontypeammo :RifleType "/Game/Items/GameActor/Weapons/PickUpFX/Bottom01-01.Bottom01-01" :ShotGunType "/Game/Items/GameActor/Weapons/PickUpFX/Bottom03-03.Bottom03-03" :GrenadeLauncher "/Game/Items/GameActor/Weapons/PickUpFX/Bottom05-05.Bottom05-05"))
  (Utilities|FlowControl|Sequence
    (:then_0
      (Utilities|IsValid 0
        (:Is%20Valid
          (Components|StaticMesh|SetStaticMesh _staticmesh (Utilities|Select :Index _weapontypeammo :RifleType "/Game/Items/GameActor/Weapons/AssaultRifle_Pickup.AssaultRifle_Pickup" :ShotGunType "/Game/Items/GameActor/Weapons/Shotgun_Pickup.Shotgun_Pickup" :GrenadeLauncher "/Game/Items/GameActor/Weapons/GrenadeLauncher_Pickup.GrenadeLauncher_Pickup"))
          (Transformation|SetRelativeLocation _staticmesh "0, 0, 0" false false)
          (Transformation|SetRelativeScale3D _staticmesh "2.000000,2.000000,2.000000")
          (Transformation|SetRelativeRotation _staticmesh (Math|Rotator|MakeRotator 0.0 0.0 0.0) false false))
        (:Is%20Not%20Valid
          (Components|DestroyComponent _staticmesh))))
    (:then_1
      (Utilities|IsValid _returnvalue
        (:Is%20Valid
          (Class|NiagaraComponent|SetAsset _niagara _returnvalue true)
          (Transformation|SetRelativeScale3D _niagara "1.000000,1.000000,1.000000"))
        (:Is%20Not%20Valid
          (Components|DestroyComponent _niagara))))))