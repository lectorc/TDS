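; A weapon pickup actor that extends a parent pickup class and takes its weapon info from the data passed to InitActor.
; On character overlap it prints a debug "Hello" and tries to add the weapon to the inventory, reporting pickup success if that works.
; If the inventory refuses it, the owning TopDown character starts a weapon switch with this pickup, which ends when that character leaves the sphere.
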(event OnComponentEndOverlap(Sphere1)
  (params (OverlappedComponent :type Primitive%20Component%20Object%20Reference) (OtherActor :type Actor%20Object%20Reference) (OtherComp :type Primitive%20Component%20Object%20Reference) (OtherBodyIndex :type Integer))
  (bind _asbp_top_down_character (Utilities|Casting|CastToBP_TopDownCharacter OtherActor))
  (Default|EndSwitchWeapon _asbp_top_down_character))

(event EventBeginPlay
  (|CallParentFunction) ; This node is disabled and will not be called.\nDrag off pins to build functionality.
)

(event EventTick
  (params (DeltaSeconds :type Float%20%28single-precision%29))
  (|CallParentFunction DeltaSeconds) ; This node is disabled and will not be called.\nDrag off pins to build functionality.
)

(event EventOverlapCharacter
  (params (ToInventory :type TDS123%20Inventory%20Component%20Object%20Reference))
  (|CallParentFunction ToInventory)
  (Development|PrintText "Hello")
  (bind _returnvalue (Class|TDS123InventoryComponent|TryGetWeapontoInventory ToInventory (Variables|Default|GetWeaponInfo_0)))
  (if _returnvalue
    (CallFunction|PickUpSuccess)
    (else
      (bind _asbp_top_down_character (Utilities|Casting|CastToBP_TopDownCharacter (Components|GetOwner ToInventory)))
      (Default|StartSwitchWeapon _asbp_top_down_character self))))

(fn ConstructionScript
  (|CallParentFunction))

(fn InitActor
  (params (InfoActor :type Drop%20Item%20Structure))
  (Variables|Default|SetWeaponInfo_0 (.WeaponInfo (Utilities|Struct|BreakDropItem InfoActor)))
  (|CallParentFunction InfoActor))