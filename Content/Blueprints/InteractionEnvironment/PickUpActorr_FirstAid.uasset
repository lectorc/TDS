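; First aid pickup actor that heals a character who overlaps it.
; On overlap it runs the parent handler, then casts the inventory component's owner to TDS123Character.
; If that character's health component reports current health below a hard-coded 100, it changes health by Value and calls PickUpSuccess.
; Otherwise, neither the heal nor PickUpSuccess runs.
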(event EventOverlapCharacter
  (params (ToInventory :type TDS123%20Inventory%20Component%20Object%20Reference))
  (|CallParentFunction ToInventory)
  (bind _astds123character (Utilities|Casting|CastToTDS123Character (Components|GetOwner ToInventory)))
  (bind _returnvalue (Class|TDS123HealthComponent|GetCurrentHealth (Variables|/Script/TDS123.TDS123Character|GetCharHealthComponent _astds123character)))
  (if (< _returnvalue 1e+02)
    (Class|TDS123HealthComponent|ChangeHealthValue (Variables|/Script/TDS123.TDS123Character|GetCharHealthComponent _astds123character) (Variables|Default|GetValue))
    (CallFunction|PickUpSuccess)))

(fn ConstructionScript
  (|CallParentFunction))